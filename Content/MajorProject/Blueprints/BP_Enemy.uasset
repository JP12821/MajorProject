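; Enemy that takes elemental damage, dies and respawns in place, serving as a lock-on target for BP_ThirdPersonCharacter.
; RecieveDamage clamps Health and updates the health bar material; at zero it plays a death animation and clears the player's pointer.
; Timelines drive the mesh's dissolve and return alongside Niagara effects, with the death fade tinted by element.
; A sphere overlap sets the player's InRange flag and breaks lock-on upon exit.
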(event `Respawn`
  (params (Delay :type "Float (double-precision)"))
  (bind _fadeaway (`self.FadeAway`))
  (`SkeletalMeshComponent.PlayAnimation` (`self.SkeletalMesh`) "/Game/MajorProject/Animations/Enemy/Idle_Anim.Idle_Anim" true)
  (`KismetSystemLibrary.Delay` Delay)
  (set `self.Health` 100.0)
  (`MeshComponent.SetScalarParameterValueOnMaterials` (`self.HealthBar`) "Min" (`KismetMathLibrary.Lerp` 0.9 0.125 (/ (`self.Health`) 100.0)))
  (`ActorComponent.Activate` _fadeaway true)
  (`ActorComponent.Activate` (`self.Spawn`) true)
  (`FXSystemComponent.SetBoolParameter` _fadeaway "Reverse?" true)
  (`KismetSystemLibrary.Delay` 0.2)
  (`SceneComponent.SetVisibility` (`self.HealthBar`) true false)
  (bind (_direction _fade) (`Timeline|Timeline_0` :!via `PlayFromStart`)
    (:`Update`
      (`MeshComponent.SetScalarParameterValueOnMaterials` (`self.SkeletalMesh`) "Fade" _fade))
    (:`Finished`
      (`KismetSystemLibrary.Delay` 3.0))))

(event `EnemyDies`
  ;[0 0.06276 0.15 0.5 40] Enemy Dies - Plays fade away VFX
  (bind _returnvalue (`GameplayStatics.GetActorOfClass` "/Game/ThirdPerson/Blueprints/BP_ThirdPersonCharacter.BP_ThirdPersonCharacter_C"))
  (`/Game/ThirdPerson/Blueprints/BP_ThirdPersonCharacter.DestroyPointer` _returnvalue)
  (`SkeletalMeshComponent.PlayAnimation` (`self.SkeletalMesh`) "/Game/MajorProject/Animations/Enemy/Death/Standing_React_Death_Backward_Anim1.Standing_React_Death_Backward_Anim1" false)
  (`ActorComponent.Activate` (`self.FadeAway`) true)
  (`self.SetFadeColour` (stale `RecieveDamage` ElementIndex))
  (bind (_direction _fade) (`Timeline|Timeline` :!via `PlayFromStart`)
    (:`Update`
      (`MeshComponent.SetScalarParameterValueOnMaterials` (`self.SkeletalMesh`) "Fade" _fade))
    (:`Finished`
      (`KismetSystemLibrary.Delay` 0.0)
      (`SceneComponent.SetVisibility` (`self.HealthBar`) false false)
      (`self.Respawn` 2.0))))

(event `CheckDamage`
  (`MeshComponent.SetScalarParameterValueOnMaterials` (`self.HealthBar`) "Min" (`KismetMathLibrary.Lerp` 0.9 0.125 (/ (`self.Health`) 100.0)) :!label _label)
  (if (== (`self.Health`) 0.0)
    (`self.EnemyDies`)
    (bind _returnvalue (`GameplayStatics.GetActorOfClass` "/Game/ThirdPerson/Blueprints/BP_ThirdPersonCharacter.BP_ThirdPersonCharacter_C"))
    (`/Game/ThirdPerson/Blueprints/BP_ThirdPersonCharacter.PointerSwitch` _returnvalue 1)))

(event `RecieveDamage`
  (params (Amount :type "Float (double-precision)") (ElementIndex :type "Float (double-precision)"))
  (set `self.Health` (`KismetMathLibrary.FClamp` (- (`self.Health`) Amount) 0.0 100.0))
  (goto _label))

(event `SetFadeColour`
  (params (ElementIndex :type "Float (double-precision)"))
  (bind _output (`|GetArrayItem` (`self.Colours`) (`KismetMathLibrary.FTrunc` ElementIndex)))
  (`NiagaraComponent.SetNiagaraVariableLinearColor` (`self.FadeAway`) "Colour" _output)
  (`MeshComponent.SetVectorParameterValueOnMaterials` (`self.SkeletalMesh`) "Colour" (`KismetMathLibrary.Conv_LinearColorToVector` _output)))

(event `self.ReceiveBeginPlay`
  (`self.CheckDamage`)
  (bind _returnvalue (`GameplayStatics.GetActorOfClass` "/Game/ThirdPerson/Blueprints/BP_ThirdPersonCharacter.BP_ThirdPersonCharacter_C"))
  (set `/Game/ThirdPerson/Blueprints/BP_ThirdPersonCharacter.InRange` true _returnvalue)
  (`self.Respawn` 0.0))

(event `self.ReceiveTick`
  (params (DeltaSeconds :type "Float (single-precision)")))

(event `self.Sphere.OnComponentBeginOverlap`
  (params (OverlappedComponent :type "PrimitiveComponent Object Reference") (OtherActor :type "Actor Object Reference") (OtherComp :type "PrimitiveComponent Object Reference") (OtherBodyIndex :type Integer) (bFromSweep :type Boolean) (SweepResult :type "HitResult Structure (by ref)"))
  (bind _asbp_third_person_character (cast `/Game/ThirdPerson/Blueprints/BP_ThirdPersonCharacter` OtherActor))
  (set `/Game/ThirdPerson/Blueprints/BP_ThirdPersonCharacter.InRange` true _asbp_third_person_character))

(event `self.Sphere.OnComponentEndOverlap`
  (params (OverlappedComponent :type "PrimitiveComponent Object Reference") (OtherActor :type "Actor Object Reference") (OtherComp :type "PrimitiveComponent Object Reference") (OtherBodyIndex :type Integer))
  (bind _asbp_third_person_character (cast `/Game/ThirdPerson/Blueprints/BP_ThirdPersonCharacter` OtherActor))
  (set `/Game/ThirdPerson/Blueprints/BP_ThirdPersonCharacter.InRange` false _asbp_third_person_character)
  (if (`/Game/ThirdPerson/Blueprints/BP_ThirdPersonCharacter.LockedIn` _asbp_third_person_character)
    (`self.K2_DestroyActor` (`/Game/ThirdPerson/Blueprints/BP_ThirdPersonCharacter.PointerLockOn` _asbp_third_person_character))
    (set `/Game/ThirdPerson/Blueprints/BP_ThirdPersonCharacter.LockedIn` false _asbp_third_person_character)))

(event `self.Capsule.OnComponentBeginOverlap`
  (params (OverlappedComponent :type "PrimitiveComponent Object Reference") (OtherActor :type "Actor Object Reference") (OtherComp :type "PrimitiveComponent Object Reference") (OtherBodyIndex :type Integer) (bFromSweep :type Boolean) (SweepResult :type "HitResult Structure (by ref)")))

(event `self.Capsule.OnComponentHit`
  (params (HitComponent :type "PrimitiveComponent Object Reference") (OtherActor :type "Actor Object Reference") (OtherComp :type "PrimitiveComponent Object Reference") (NormalImpulse :type "Vector Structure") (Hit :type "HitResult Structure (by ref)")))

(fn `UserConstructionScript`)