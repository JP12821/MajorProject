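; BP_Charge is a projectile charge effect actor tinted to match the player character's element.
; Its construction script finds BP_Character and uses the truncated Element value to index its Colours array, setting the Colour variable on the Projectile effect component.
; Tick adds a fixed step to a Time counter each frame, independent of delta time, with no use of it in this file.
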(event `self.ReceiveTick`
  (params (DeltaSeconds :type "Float (single-precision)"))
  (set `self.Time` (+ (`self.Time`) 0.1)))

(fn `UserConstructionScript`
  (bind _returnvalue (`GameplayStatics.GetActorOfClass` "/Game/MajorProject/BP_Character.BP_Character_C"))
  (`NiagaraComponent.SetVariableLinearColor` (`self.Projectile`) "Colour" (`|GetArrayItem` (`/Game/MajorProject/BP_Character.Colours` _returnvalue) (`KismetMathLibrary.FTrunc` (`/Game/MajorProject/BP_Character.Element` _returnvalue)))))