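; BP_Projectile is an elemental spell projectile built on a Niagara system that damages BP_Enemy actors.
; Construction picks a normal or combo effect by ElementIndex and feeds it rotation, level and distance, with one combo raised to fall downward.
; On BeginPlay it sets the Kill flag on other projectiles.
; Particle positions exported back from Niagara serve as collision, applying Level-scaled elemental damage once to a nearby enemy.
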(event `self.ReceiveParticleData`
  (params (Data :type "Array of BasicParticleData Structure (by ref)") (NiagaraSystem :type "NiagaraSystem Object Reference") (SimulationPositionOffset :type "Vector Structure (by ref)"))
  (bind _returnvalue (* (`self.Level`) 20.0))
  ; Collision form Niagara passed into enemy for damage
  (`KismetSystemLibrary.PrintString` "recieved")
  (for _array_element Data
    (bind _outactors (`GameplayStatics.GetAllActorsOfClass` "/Game/MajorProject/Blueprints/BP_Enemy.BP_Enemy_C"))
    (for _array_element_2 _outactors
      (if (< (`KismetMathLibrary.Vector_Distance` (`SceneComponent.K2_GetComponentLocation` (`/Game/MajorProject/Blueprints/BP_Enemy.Capsule` _array_element_2)) (`.Position` (break `BasicParticleData` _array_element))) 100.0)
        (`/Engine/EditorBlueprintResources/StandardMacros.DoOnce` false
          (:`Completed`
            (`KismetSystemLibrary.PrintString` "ouch")
            (`/Game/MajorProject/Blueprints/BP_Enemy.RecieveDamage` _array_element_2 _returnvalue (`self.ElementIndex`))
            (`KismetSystemLibrary.PrintString` (`KismetStringLibrary.Conv_DoubleToString` _returnvalue))))))))

(event `self.ReceiveBeginPlay`
  (`NiagaraComponent.SetVariableActor` (`self.Projectile`) "Blueprint" self)
  (bind _outactors (`GameplayStatics.GetAllActorsOfClass` "BP_Projectile_C"))
  (for _array_element _outactors
    (`NiagaraComponent.SetNiagaraVariableBool` (`/Game/MajorProject/Blueprints/Projectile/BP_Projectile.Projectile` _array_element) "Kill" (!= _array_element self))))

(event `self.ReceiveTick`
  (params (DeltaSeconds :type "Float (single-precision)")))

(fn `UserConstructionScript`
  (bind _projectile (`self.Projectile`))
  (bind _rotation (`self.Rotation`))
  (bind (_returnvalue_x _returnvalue_y _returnvalue_z) (`KismetMathLibrary.BreakVector` (`SceneComponent.K2_GetComponentLocation` (`self.Projectile`))))
  (bind _returnvalue (* (`self.Distance`) 120.0))
  ; Creation of projectile using passed parameters
  (if (`self.Combo?`)
    (`NiagaraComponent.SetAsset` (`self.Projectile`) (`|GetArrayItem` (`self.NiagaraSpecial`) (`KismetMathLibrary.FTrunc` (- (`self.ElementIndex`) 1.0))) true)
    (if (== (`self.ElementIndex`) 6.0)
      (`SceneComponent.K2_SetWorldLocation` (`self.Projectile`) (`KismetMathLibrary.MakeVector` _returnvalue_x _returnvalue_y (+ _returnvalue_z 300.0)) false false)
      (`NiagaraComponent.SetVariableFloat` (`self.Projectile`) "DownwardVelocity" -1000.0))
    (else
      (`NiagaraComponent.SetAsset` (`self.Projectile`) (`|GetArrayItem` (`self.Niagara`) (`KismetMathLibrary.FTrunc` (- (`self.ElementIndex`) 1.0))) true)))
  (`NiagaraComponent.SetVariableFloat` _projectile "Rotation" _rotation)
  (`NiagaraComponent.SetVariableFloat` _projectile "Level" (`self.Level`))
  (`NiagaraComponent.SetVariableFloat` _projectile "ProjectileRotation" _rotation)
  (`NiagaraComponent.SetVariableFloat` (`self.Projectile`) "Offset" _returnvalue)
  (`KismetSystemLibrary.PrintString` (`KismetStringLibrary.Conv_DoubleToString` _returnvalue))
  (`NiagaraComponent.SetVariableFloat` (`self.Projectile`) "Distance" (/ (`self.Distance`) (`self.Level`))))