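; BP_SkullAttack is a short-lived attack actor with a Niagara effect that damages the player's locked-on enemy.
; Its construction script finds BP_Character and, if that character is locked on, caches the lock-on target.
; Tick uses chained Delays to apply elemental damage after a wind-up, then destroys the actor just before the first Delay would fire again.
; Without a target, it neither deals damage nor destroys itself in this graph.
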(event `self.ReceiveTick`
  (params (DeltaSeconds :type "Float (single-precision)"))
  (`KismetSystemLibrary.Delay` 2.0)
  (if (`self.LockedIn`)
    (`/Game/MajorProject/Blueprints/BP_Enemy.RecieveDamage` (`self.EnemyHit`) 20.0 7.0)
    (`KismetSystemLibrary.Delay` 1.9)
    (`self.K2_DestroyActor`)))

(event `self.Niagara.OnSystemFinished`
  (params (PSystem :type "NiagaraComponent Object Reference")))

(fn `UserConstructionScript`
  (bind _returnvalue (`GameplayStatics.GetActorOfClass` "/Game/MajorProject/BP_Character.BP_Character_C"))
  (if (`/Game/MajorProject/BP_Character.LockedIn` _returnvalue)
    (set `self.EnemyHit` (`/Game/MajorProject/BP_Character.EnemyLockOn` _returnvalue))
    (set `self.LockedIn` true)))