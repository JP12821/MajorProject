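; Menu actor that switches between four Niagara effects tied to the Play, Controls, Info and Quit options.
; Its SetEmitter event sets the Kill variable on all four systems, then clears it on the one matching the float index it receives.
; Only the selected option's effect stays active, and an unmatched index leaves all four killed.
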(event `Set Emitter`
  (params (Float :type "Float (double-precision)"))
  (`NiagaraComponent.SetVariableBool` (`self.NS_Play`) "Kill" true)
  (`NiagaraComponent.SetVariableBool` (`self.NS_Quit`) "Kill" true)
  (`NiagaraComponent.SetVariableBool` (`self.NS_Info`) "Kill" true)
  (`NiagaraComponent.SetVariableBool` (`self.NS_Controls`) "Kill" true)
  (if (== Float 1.0)
    (`NiagaraComponent.SetVariableBool` (`self.NS_Play`) "Kill" false)
    (elif (== Float 2.0)
      (`NiagaraComponent.SetVariableBool` (`self.NS_Controls`) "Kill" false)
      (elif (== Float 3.0)
        (`NiagaraComponent.SetVariableBool` (`self.NS_Info`) "Kill" false)
        (elif (== Float 4.0)
          (`NiagaraComponent.SetVariableBool` (`self.NS_Quit`) "Kill" false))))))

(fn `UserConstructionScript`)