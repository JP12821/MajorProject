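; BP_Laser is a laser hazard with a Niagara beam that electrocutes the player character when tripped.
; The construction script passes Vector1, Vector2 and Kill to the Niagara effect.
; Each Tick it line-traces on Visibility between those offsets from the effect's location, with persistent debug drawing.
; Any hit prints a debug string, plays an electrocution animation on BP_ThirdPersonCharacter and calls DisableInput, without checking the hit actor.
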(event `self.ReceiveTick`
  (params (DeltaSeconds :type "Float (single-precision)"))
  (bind _returnvalue (`SceneComponent.K2_GetComponentLocation` (`self.Laser`)))
  (bind (_outhit _returnvalue_2) (`KismetSystemLibrary.LineTraceSingle` :`Start` (+ (`self.Vector1`) _returnvalue) :`End` (+ _returnvalue (`self.Vector2`)) :`TraceChannel` "TraceTypeQuery1" :`bTraceComplex` true :`DrawDebugType` "Persistent"))
  (if _returnvalue_2
    (`KismetSystemLibrary.PrintString` "n")
    (bind _returnvalue_3 (`GameplayStatics.GetActorOfClass` "/Game/ThirdPerson/Blueprints/BP_ThirdPersonCharacter.BP_ThirdPersonCharacter_C"))
    (`SkeletalMeshComponent.PlayAnimation` (`Character.Mesh` _returnvalue_3) "/Game/MajorProject/Animations/Electrocuted/Being_Electrocuted__1__Anim1_Montage.Being_Electrocuted__1__Anim1_Montage" false)
    (`self.DisableInput` null)))

(fn `UserConstructionScript`
  (`NiagaraComponent.SetNiagaraVariableVec3` (`self.Laser`) "Vector1" (`self.Vector1`))
  (`NiagaraComponent.SetNiagaraVariableVec3` (`self.Laser`) "Vector2" (`self.Vector2`))
  (`NiagaraComponent.SetVariableBool` (`self.Laser`) "Kill" (`self.Kill`)))