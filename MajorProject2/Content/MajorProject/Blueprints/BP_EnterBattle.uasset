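; Trigger volume that moves the third-person character into a battle when it enters the box.
; Beginning overlap sets the character's InRange flag and, only once, plays the LS_Battle sequence.
; After a fixed delay matched to that sequence, it switches the view to Camera and moves the character to a hardcoded location and rotation.
; Ending overlap clears InRange and removes any active lock-on pointer.
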(event `self.Box.OnComponentBeginOverlap`
  (params (OverlappedComponent :type "PrimitiveComponent Object Reference") (OtherActor :type "Actor Object Reference") (OtherComp :type "PrimitiveComponent Object Reference") (OtherBodyIndex :type Integer) (bFromSweep :type Boolean) (SweepResult :type "HitResult Structure (by ref)"))
  (bind _asbp_third_person_character (cast `/Game/ThirdPerson/Blueprints/BP_ThirdPersonCharacter` OtherActor))
  (set `/Game/ThirdPerson/Blueprints/BP_ThirdPersonCharacter.InRange` true _asbp_third_person_character)
  (`/Engine/EditorBlueprintResources/StandardMacros.DoOnce` false
    (:`Completed`
      (bind (_outactor _returnvalue) (`LevelSequencePlayer.CreateLevelSequencePlayer` "/Game/MajorProject/LevelSequences/LS_Battle.LS_Battle"))
      (`MovieSceneSequencePlayer.Play` _returnvalue)
      (`KismetSystemLibrary.Delay` 3.02)
      (`PlayerController.SetViewTargetWithBlend` (`GameplayStatics.GetPlayerController` 0) (`self.Camera`) 0.0 "VTBlend_Linear" 0.0 false)
      (`self.K2_SetActorLocation` _asbp_third_person_character (1000.0 1000.0 100.0) false false)
      (`self.K2_SetActorRotation` :`self` _asbp_third_person_character))))

(event `self.Box.OnComponentEndOverlap`
  (params (OverlappedComponent :type "PrimitiveComponent Object Reference") (OtherActor :type "Actor Object Reference") (OtherComp :type "PrimitiveComponent Object Reference") (OtherBodyIndex :type Integer))
  (bind _asbp_third_person_character (cast `/Game/ThirdPerson/Blueprints/BP_ThirdPersonCharacter` OtherActor))
  (set `/Game/ThirdPerson/Blueprints/BP_ThirdPersonCharacter.InRange` false _asbp_third_person_character)
  (if (`/Game/ThirdPerson/Blueprints/BP_ThirdPersonCharacter.LockedIn` _asbp_third_person_character)
    (`self.K2_DestroyActor` (`/Game/ThirdPerson/Blueprints/BP_ThirdPersonCharacter.PointerLockOn` _asbp_third_person_character))
    (set `/Game/ThirdPerson/Blueprints/BP_ThirdPersonCharacter.LockedIn` false _asbp_third_person_character)))

(fn `UserConstructionScript`)