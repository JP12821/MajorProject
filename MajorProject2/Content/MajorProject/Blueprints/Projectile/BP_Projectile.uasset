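; BP_Projectile is a projectile whose Niagara effect drives hit detection against enemies.
; The construction script picks a phoenix, skull or ice system from ElementIndex, offsetting rotation for the skull.
; BeginPlay passes the actor to Niagara, whose exported particle positions are distance-checked against every BP_Enemy capsule.
; A single DoOnce limits it to one fixed-damage hit, with debug prints left in and spawn and destroy logic unconnected.
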(event `self.ReceiveTick`
  (params (DeltaSeconds :type "Float (single-precision)")))

(event `self.ReceiveParticleData`
  (params (Data :type "Array of BasicParticleData Structure (by ref)") (NiagaraSystem :type "NiagaraSystem Object Reference") (SimulationPositionOffset :type "Vector Structure (by ref)"))
  (`KismetSystemLibrary.PrintString` "sss")
  (for _array_element Data
    (bind _outactors (`GameplayStatics.GetAllActorsOfClass` "/Game/MajorProject/Blueprints/BP_Enemy.BP_Enemy_C"))
    (for _array_element_2 _outactors
      (if (< (`KismetMathLibrary.Vector_Distance` (`SceneComponent.K2_GetComponentLocation` (`/Game/MajorProject/Blueprints/BP_Enemy.Capsule` _array_element_2)) (`.Position` (break `BasicParticleData` _array_element))) 100.0)
        (`/Engine/EditorBlueprintResources/StandardMacros.DoOnce` false
          (:`Completed`
            (`KismetSystemLibrary.PrintString` "ouch")
            (`/Game/MajorProject/Blueprints/BP_Enemy.RecieveDamage` _array_element_2 20.0)))))))

(event `self.ReceiveBeginPlay`
  (`NiagaraComponent.SetVariableActor` (`self.Projectile`) "Blueprint" self))

(fn `UserConstructionScript`
  (bind _projectile (`self.Projectile`))
  (if (== (`self.ElementIndex`) 6.0)
    (`NiagaraComponent.SetAsset` (`self.Projectile`) "/Game/MajorProject/Niagara/Projectiles/NS_ProjectilePheonix.NS_ProjectilePheonix" true)
    (elif (== (`self.ElementIndex`) 7.0)
      (`NiagaraComponent.SetAsset` _projectile "/Game/MajorProject/Niagara/NS_SkullAttack3.NS_SkullAttack3" true)
      (`NiagaraComponent.SetVariableFloat` _projectile "Rotation" (- (`self.Rotation`) 90.0))
      (elif (== (`self.ElementIndex`) 2.0)
        (`NiagaraComponent.SetAsset` (`self.Projectile`) "/Game/MajorProject/Niagara/Projectiles/NS_Ice.NS_Ice" true)))))