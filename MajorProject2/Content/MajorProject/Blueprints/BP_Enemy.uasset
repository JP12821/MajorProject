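; Enemy actor Blueprint with health, a material-driven health bar, and a range sphere for the player's lock-on.
; RecieveDamage clamps Health and shares CheckDamage's logic, which also runs on BeginPlay to update the bar's "Min" parameter.
; At zero health it plays a death animation, activates FadeAway, hides the bar and destroys itself after a delay.
; Sphere overlaps toggle BP_ThirdPersonCharacter's InRange; leaving also clears any active lock-on and destroys its pointer.
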(event `CheckDamage`
  (`MeshComponent.SetScalarParameterValueOnMaterials` (`self.HealthBar`) "Min" (`KismetMathLibrary.Lerp` 0.9 0.125 (/ (`self.Health`) 100.0)) :!label _label)
  (if (== (`self.Health`) 0.0)
    (`SkeletalMeshComponent.PlayAnimation` (`self.SkeletalMesh`) "/Game/MajorProject/Animations/Enemy/Death/Standing_React_Death_Backward_Anim1.Standing_React_Death_Backward_Anim1" false)
    (`ActorComponent.Activate` (`self.FadeAway`) false)
    (`KismetSystemLibrary.Delay` 0.2)
    (`SceneComponent.SetVisibility` (`self.HealthBar`) false false)
    (`KismetSystemLibrary.Delay` 3.0)
    (`self.K2_DestroyActor`)))

(event `RecieveDamage`
  (params (Amount :type "Float (double-precision)"))
  (set `self.Health` (`KismetMathLibrary.FClamp` (- (`self.Health`) Amount) 0.0 100.0))
  (goto _label))

(event `self.ReceiveBeginPlay`
  (`self.CheckDamage`))

(event `self.ReceiveTick`
  (params (DeltaSeconds :type "Float (single-precision)")))

(event `self.Sphere.OnComponentBeginOverlap`
  (params (OverlappedComponent :type "PrimitiveComponent Object Reference") (OtherActor :type "Actor Object Reference") (OtherComp :type "PrimitiveComponent Object Reference") (OtherBodyIndex :type Integer) (bFromSweep :type Boolean) (SweepResult :type "HitResult Structure (by ref)"))
  (bind _asbp_third_person_character (cast `/Game/ThirdPerson/Blueprints/BP_ThirdPersonCharacter` OtherActor))
  (set `/Game/ThirdPerson/Blueprints/BP_ThirdPersonCharacter.InRange` true _asbp_third_person_character))

(event `self.Sphere.OnComponentEndOverlap`
  (params (OverlappedComponent :type "PrimitiveComponent Object Reference") (OtherActor :type "Actor Object Reference") (OtherComp :type "PrimitiveComponent Object Reference") (OtherBodyIndex :type Integer))
  (bind _asbp_third_person_character (cast `/Game/ThirdPerson/Blueprints/BP_ThirdPersonCharacter` OtherActor))
  (set `/Game/ThirdPerson/Blueprints/BP_ThirdPersonCharacter.InRange` false _asbp_third_person_character)
  (if (`/Game/ThirdPerson/Blueprints/BP_ThirdPersonCharacter.LockedIn` _asbp_third_person_character)
    (`self.K2_DestroyActor` (`/Game/ThirdPerson/Blueprints/BP_ThirdPersonCharacter.PointerLockOn` _asbp_third_person_character))
    (set `/Game/ThirdPerson/Blueprints/BP_ThirdPersonCharacter.LockedIn` false _asbp_third_person_character)))

(event `self.Capsule.OnComponentBeginOverlap`
  (params (OverlappedComponent :type "PrimitiveComponent Object Reference") (OtherActor :type "Actor Object Reference") (OtherComp :type "PrimitiveComponent Object Reference") (OtherBodyIndex :type Integer) (bFromSweep :type Boolean) (SweepResult :type "HitResult Structure (by ref)")))

(event `self.Capsule.OnComponentHit`
  (params (HitComponent :type "PrimitiveComponent Object Reference") (OtherActor :type "Actor Object Reference") (OtherComp :type "PrimitiveComponent Object Reference") (NormalImpulse :type "Vector Structure") (Hit :type "HitResult Structure (by ref)")))

(fn `UserConstructionScript`)